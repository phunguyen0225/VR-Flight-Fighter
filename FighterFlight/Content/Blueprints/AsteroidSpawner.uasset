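; Spawner actor that emits moving asteroids at its own transform at random intervals of a few seconds while spawning is enabled.
; Tick runs a random Delay and then calls SpawnAsteroid, which creates an asteroid only while the VR game mode has not flagged a loss.
; Each new asteroid receives the spawner's Ship and Score references.
; Two custom events turn spawning off or toggle it.
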(event `self.ReceiveTick`
  (params (DeltaSeconds :type "Float (single-precision)"))
  (if (`self.spawning`)
    (`KismetSystemLibrary.Delay` (`KismetMathLibrary.RandomFloatInRange` 2.0 4.0))
    (`self.Spawn Asteroid`)))

(event `Spawn Asteroid`
  (bind _asvrgame_mode (cast `/Game/VRTemplate/Blueprints/VRGameMode` (`GameplayStatics.GetGameMode`)))
  (if (not (`/Game/VRTemplate/Blueprints/VRGameMode.IsLose?` _asvrgame_mode))
    (bind _returnvalue (`|SpawnActorFromClass` "/Game/Blueprints/Moving_Asteroid.Moving_Asteroid_C" (`self.GetTransform`) "AdjustIfPossibleButAlwaysSpawn" "OverrideRootScale" null null))
    (set `/Game/Blueprints/Moving_Asteroid.Ship` (`self.Ship`) _returnvalue)
    (set `/Game/Blueprints/Moving_Asteroid.Score` (`self.Score`) _returnvalue)))

(event `Don't SPawn`
  (set `self.spawning` false))

(event `Switchspawning`
  (if (`self.spawning`)
    (set `self.spawning` false)
    (else
      (set `self.spawning` true))))

(fn `UserConstructionScript`)