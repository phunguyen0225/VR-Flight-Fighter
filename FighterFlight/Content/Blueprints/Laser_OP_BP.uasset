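; Cyan laser beam actor that damages Destructible-tagged enemies and missiles, destroyed by server or client end-beam events.
; Tick line-traces forward to place the Niagara beam end and impact effect, clamping length on hits and rapidly regrowing it toward MaxDistance.
; Damage comes from actor overlap, not the trace, repeating every 0.2 seconds while a shared IsDamaging flag holds.
; Only an Enemy_Base ending overlap clears that flag; missiles never do.
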(event `Server End Beam`
  (`self.K2_DestroyActor` :!label _label))

(event `self.ReceiveBeginPlay`
  (`FXSystemComponent.SetColorParameter` (`self.NiagaraLaser`) "Color" (struct :`G` 0.850594 :`B` 1.0 :`A` 1.0))
  (`FXSystemComponent.SetColorParameter` (`self.NiagaraLaserImpact`) "Color" (struct :`G` 0.850594 :`B` 1.0 :`A` 1.0)))

(event `Client End Beam`
  (goto _label))

(event `self.ReceiveActorBeginOverlap`
  (params (OtherActor :type "Actor Object Reference"))
  (bind _damage (`self.Damage`))
  (if (`self.ActorHasTag` OtherActor "Destructible")
    (bind _asenemy_base (cast `/Game/Blueprints/Enemy_Base` OtherActor)
      (:`then`
        (set `self.IsDamaging` true)
        (`/Game/Blueprints/Enemy_Base.Damage Rock` _asenemy_base _damage :!label _label_2)
        (`KismetSystemLibrary.Delay` 0.2)
        (if (`self.IsDamaging`)
          (goto _label_2)))
      (:`CastFailed`
        (bind _asenemy_missile (cast `/Game/Blueprints/Enemy_Missile` OtherActor))
        (set `self.IsDamaging` true)
        (`/Game/Blueprints/Enemy_Missile.TakeDamage` _asenemy_missile _damage :!label _label_3)
        (`KismetSystemLibrary.Delay` 0.2)
        (if (`self.IsDamaging`)
          (goto _label_3))))))

(event `self.ReceiveActorEndOverlap`
  (params (OtherActor :type "Actor Object Reference"))
  (if (`self.ActorHasTag` OtherActor "Destructible")
    (cast `/Game/Blueprints/Enemy_Base` OtherActor)
    (set `self.IsDamaging` false)))

(event `self.ReceiveTick`
  (params (DeltaSeconds :type "Float (single-precision)"))
  (bind _returnvalue (`self.K2_GetActorLocation`))
  (bind _returnvalue_2 (+ _returnvalue (* (`self.GetActorForwardVector`) (`self.Distance`))))
  (`|ExecutionSequence`
    (:`then_0`
      (set `self.TraceEnd` _returnvalue_2)
      (bind _outhit (`KismetSystemLibrary.LineTraceSingle` _returnvalue _returnvalue_2 "TraceTypeQuery1"))
      (bind (_bblockinghit _binitialoverlap _time _distance _location) (`GameplayStatics.BreakHitResult` _outhit))
      (set `self.bHit` _bblockinghit)
      (set `self.HitLocation` _location)
      (`FXSystemComponent.SetVectorParameter` (`self.NiagaraLaser`) "LaserEnd" (select `bool` (`self.bHit`) :`false` (`self.TraceEnd`) :`true` (`self.HitLocation`)))
      (`SceneComponent.SetVisibility` (`self.NiagaraLaserImpact`) (`self.bHit`) false)
      (`SceneComponent.K2_SetWorldLocation` (`self.NiagaraLaserImpact`) (`self.HitLocation`) false false)
      (if (`self.bHit`)
        (set `self.Distance` (`KismetMathLibrary.VSize` (- (`self.HitLocation`) (`self.K2_GetActorLocation`))))))
    (:`then_1`
      (if (< (`self.Distance`) (`self.MaxDistance`))
        (set `self.Distance` (+ (`self.Distance`) (* DeltaSeconds 100000000.0)))))))

(fn `UserConstructionScript`)