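; Super charge blast actor, likely a projectile, that detonates on contact with destructible enemies.
; When its sphere collision overlaps an Enemy_Base actor tagged Destructible, it spawns a greatly enlarged Explosion_BP at the sphere's transform and destroys itself.
; It passes its ChargeScale to the explosion as ChargeFactor and prints a leftover debug string.
; A delay from BeginPlay destroys it after a few seconds if nothing is hit.
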(event `self.SphereCollision.OnComponentBeginOverlap`
  (params (OverlappedComponent :type "PrimitiveComponent Object Reference") (OtherActor :type "Actor Object Reference") (OtherComp :type "PrimitiveComponent Object Reference") (OtherBodyIndex :type Integer) (bFromSweep :type Boolean) (SweepResult :type "HitResult Structure (by ref)"))
  (bind _spherecollision (`self.SphereCollision`))
  (if (`self.ActorHasTag` OtherActor "Destructible")
    (cast `/Game/Blueprints/Enemy_Base` OtherActor)
    (`|SpawnActorFromClass` "/Game/Blueprints/Explosion_BP.Explosion_BP_C" (`KismetMathLibrary.MakeTransform` (`SceneComponent.K2_GetComponentLocation` _spherecollision) (`SceneComponent.K2_GetComponentRotation` _spherecollision) (10.0 10.0 10.0)) "Undefined" "OverrideRootScale" null (`self.ChargeScale`) null)
    (`KismetSystemLibrary.PrintString` "LESS THAN")
    (`self.K2_DestroyActor`)))

(event `self.ReceiveBeginPlay`
  (`KismetSystemLibrary.Delay` 5.0)
  (`self.K2_DestroyActor`))

(fn `UserConstructionScript`)