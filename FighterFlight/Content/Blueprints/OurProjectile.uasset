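; OurProjectile is a projectile that damages destructible asteroids and pushes physics objects it overlaps.
; When its collision sphere overlaps an actor tagged Destructible that is a Moving_Asteroid, it applies its Damage through DamageRock, spawns an explosion emitter and destroys itself.
; Any other overlapped component that simulates physics receives an impulse from the projectile's velocity, after which the projectile is destroyed without an explosion.
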(event `self.SphereCollision.OnComponentBeginOverlap`
  (params (OverlappedComponent :type "PrimitiveComponent Object Reference") (OtherActor :type "Actor Object Reference") (OtherComp :type "PrimitiveComponent Object Reference") (OtherBodyIndex :type Integer) (bFromSweep :type Boolean) (SweepResult :type "HitResult Structure (by ref)"))
  (if (`self.ActorHasTag` OtherActor "Destructible")
    (bind _asmoving_asteroid (cast `/Game/Blueprints/Moving_Asteroid` OtherActor)
      (:`then`
        ;[0.03434 0.03434 0.03434] Add a physics impulse when we hit an object that simulates physics - it's better to manually control this than it is to rely on rigid bodies colliding.
        (`/Game/Blueprints/Moving_Asteroid.Damage Rock` _asmoving_asteroid (`self.Damage`))
        (`GameplayStatics.SpawnEmitterAtLocation` "/Game/Particles/P_Explosion.P_Explosion" (`SceneComponent.K2_GetComponentLocation` (`self.SphereCollision`)))
        ;[0.03434 0.03434 0.03434] Destroy the projectile
        (`self.K2_DestroyActor` :!label _label))
      (:`CastFailed`
        (if (`SceneComponent.IsSimulatingPhysics` OtherComp "None") :!label _label_2
          (`PrimitiveComponent.AddImpulse` OtherComp (* (`MovementComponent.Velocity` (`self.ProjectileMovement`)) 1.0) "None" false)
          (goto _label))))
    (else
      (goto _label_2))))

(fn `UserConstructionScript`)