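; Enemy missile projectile that damages ShipGoalPostl actors and self-destructs after a short lifetime.
; Sphere overlap with a "Damagable"-tagged component subtracts Damage through the actor's UpdateHealth, then spawns an explosion and destroys the missile.
; Untagged physics-simulating components instead receive a velocity-based impulse before the missile is destroyed, without an explosion.
; TakeDamage is empty and a DamageRock call is left disconnected.
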(event `self.SphereCollision.OnComponentBeginOverlap`
  (params (OverlappedComponent :type "PrimitiveComponent Object Reference") (OtherActor :type "Actor Object Reference") (OtherComp :type "PrimitiveComponent Object Reference") (OtherBodyIndex :type Integer) (bFromSweep :type Boolean) (SweepResult :type "HitResult Structure (by ref)"))
  (if (`ActorComponent.ComponentHasTag` OtherComp "Damagable")
    (bind _asship_goal_postl (cast `/Game/Blueprints/ShipGoalPostl` OtherActor))
    (`/Game/Blueprints/ShipGoalPostl.Update health` _asship_goal_postl (* (`self.Damage`) -1))
    (`GameplayStatics.SpawnEmitterAtLocation` "/Game/Particles/P_Explosion.P_Explosion" (`SceneComponent.K2_GetComponentLocation` (`self.SphereCollision`)) (struct) (0.5 0.5 0.5))
    ;[0.03434 0.03434 0.03434] Destroy the projectile
    (`self.K2_DestroyActor` :!label _label)
    (else
      ;[0.03434 0.03434 0.03434] Add a physics impulse when we hit an object that simulates physics - it's better to manually control this than it is to rely on rigid bodies colliding.
      (if (`SceneComponent.IsSimulatingPhysics` OtherComp "None")
        (`PrimitiveComponent.AddImpulse` OtherComp (* (`MovementComponent.Velocity` (`self.ProjectileMovement`)) 1.0) "None" false)
        (goto _label)))))

(event `TakeDamage`
  (params (damage :type Integer)))

(event `self.ReceiveBeginPlay`
  (`KismetSystemLibrary.Delay` 4.0)
  (`self.K2_DestroyActor`))

(fn `UserConstructionScript`)