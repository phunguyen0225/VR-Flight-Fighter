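; Moving asteroid hazard in a VR game that flies at the ship and can be destroyed for points.
; On BeginPlay, after a brief delay, it aims its projectile movement at the Ship with random speed and spin.
; DamageRock reduces health, playing hit sounds or exploding and adding score, while hitting a Damagable goal post component damages that post and destroys the rock.
; A delayed Tick check destroys it once the game mode flags a loss.
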(event `Damage Rock`
  (params (Damage :type Integer))
  (bind _output_get (set `self.Health` (- (`self.Health`) Damage)))
  (if (<= _output_get 0)
    (`/Game/Blueprints/ScoreBoard.Add Score` (`self.Score`) (`self.Point Value`))
    (`GameplayStatics.SpawnSoundAtLocation` "/Game/Audio/DeepExplosion_Cue.DeepExplosion_Cue" (`SceneComponent.K2_GetComponentLocation` (`self.Sphere`)) (struct) 1.0 1.0 0.0 null null)
    (`GameplayStatics.SpawnEmitterAtLocation` "/Game/Particles/P_Explosion.P_Explosion" (`SceneComponent.K2_GetComponentLocation` (`self.Sphere`)) (struct) (2.0 2.0 2.0))
    (`self.K2_DestroyActor`)
    (else
      (`GameplayStatics.SpawnSoundAtLocation` "/Game/Audio/Explosion_Cue.Explosion_Cue" (`SceneComponent.K2_GetComponentLocation` (`self.Sphere`)) (struct) 1.0 1.0 0.0 null null))))

(event `self.SkeletalMesh.OnComponentBeginOverlap`
  (params (OverlappedComponent :type "PrimitiveComponent Object Reference") (OtherActor :type "Actor Object Reference") (OtherComp :type "PrimitiveComponent Object Reference") (OtherBodyIndex :type Integer) (bFromSweep :type Boolean) (SweepResult :type "HitResult Structure (by ref)")))

(event `self.Sphere.OnComponentBeginOverlap`
  (params (OverlappedComponent :type "PrimitiveComponent Object Reference") (OtherActor :type "Actor Object Reference") (OtherComp :type "PrimitiveComponent Object Reference") (OtherBodyIndex :type Integer) (bFromSweep :type Boolean) (SweepResult :type "HitResult Structure (by ref)"))
  ;[1 1 1] Rock hits goal post
  (bind _asship_goal_postl (cast `/Game/Blueprints/ShipGoalPostl` OtherActor))
  (if (`ActorComponent.ComponentHasTag` OtherComp "Damagable")
    (`/Game/Blueprints/ShipGoalPostl.Update health` _asship_goal_postl (* (`self.Damage Value`) -1))
    (`self.K2_DestroyActor`)))

(event `self.ReceiveBeginPlay`
  (`parent.ReceiveBeginPlay`)
  (`KismetSystemLibrary.Delay` 0.02)
  (set `MovementComponent.Velocity` (* (`KismetMathLibrary.Normal` (- (`self.K2_GetActorLocation` (`self.Ship`)) (`self.K2_GetActorLocation`))) (`KismetMathLibrary.RandomFloatInRange` 90.0 180.0)) (`self.ProjectileMovement`))
  (set `RotatingMovementComponent.RotationRate` (`KismetMathLibrary.MakeRotator` (`KismetMathLibrary.RandomFloatInRange` 10.0 90.0) (`KismetMathLibrary.RandomFloatInRange` 10.0 90.0) (`KismetMathLibrary.RandomFloatInRange` 10.0 90.0)) (`self.RotatingMovement`)))

(event `self.ReceiveTick`
  (params (DeltaSeconds :type "Float (single-precision)"))
  (`parent.ReceiveTick` DeltaSeconds)
  (`KismetSystemLibrary.Delay` 0.2)
  (bind _asvrgame_mode (cast `/Game/VRTemplate/Blueprints/VRGameMode` (`GameplayStatics.GetGameMode`)))
  (if (`/Game/VRTemplate/Blueprints/VRGameMode.IsLose?` _asvrgame_mode)
    (`self.K2_DestroyActor`)))

(fn `UserConstructionScript`
  (`parent.UserConstructionScript`))