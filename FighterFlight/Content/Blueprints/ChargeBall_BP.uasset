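; ChargeBall_BP is a charge-ball Blueprint whose scale-up-then-fire logic is present but never runs, as the Charge event is empty.
; The disconnected nodes check IsCharging, grow world scale in small steps through a short Delay that re-calls Charge, and call Fire at MaxScale or when charging stops.
; The construction script is empty.
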(event `self.Charge`)

(fn `UserConstructionScript`)