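; ShipGoalPostl is a ship goal actor that tracks health and triggers a loss in the VR game when that health runs out.
; Updatehealth adds a signed change, caps it at MaxHealth, and calls GameLose on VRGameMode at zero or below, leaving Health and display unchanged.
; Restart refills Health to MaxHealth.
; Other health changes are pushed to the ShipHealth widget hosted by the Healthtotal component.
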(event `Update health`
  (params (Modify :type Integer))
  (bind _returnvalue (+ Modify (`self.Health`)))
  (if (> _returnvalue (`self.MaxHealth`))
    (bind _output_get (set `self.Health` (`self.MaxHealth`)))
    (bind _asship_health (cast `/Game/Blueprints/ShipHealth` (`WidgetComponent.GetUserWidgetObject` (`self.healthtotal`))))
    (`/Game/Blueprints/ShipHealth.update Health` _asship_health _output_get)
    (elif (<= _returnvalue 0)
      (bind _asvrgame_mode (cast `/Game/VRTemplate/Blueprints/VRGameMode` (`GameplayStatics.GetGameMode`)))
      (`/Game/VRTemplate/Blueprints/VRGameMode.Game Lose` _asvrgame_mode)
      (else
        (bind _output_get_2 (set `self.Health` _returnvalue))
        (bind _asship_health_2 (cast `/Game/Blueprints/ShipHealth` (`WidgetComponent.GetUserWidgetObject` (`self.healthtotal`))))
        (`/Game/Blueprints/ShipHealth.update Health` _asship_health_2 _output_get_2)))))

(event `Restart`
  (bind _output_get (set `self.Health` (`self.MaxHealth`)))
  (bind _asship_health (cast `/Game/Blueprints/ShipHealth` (`WidgetComponent.GetUserWidgetObject` (`self.healthtotal`))))
  (`/Game/Blueprints/ShipHealth.update Health` _asship_health _output_get))

(fn `UserConstructionScript`)