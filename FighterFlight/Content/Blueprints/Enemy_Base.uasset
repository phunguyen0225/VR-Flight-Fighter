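; Base enemy Blueprint for a destructible rock that awards points when destroyed and damages the goal post it hits.
; DamageRock lowers health, playing an impact sound while it survives, or adding score and spawning explosion sound and particles before destroying the actor.
; Sphere overlap with a ShipGoalPostl component tagged Damagable subtracts the rock's damage value from that post's health and destroys the rock.
; The damage value's OnRep function is empty.
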(event `Damage Rock`
  (params (Damage :type Integer))
  (bind _output_get (set `self.Health` (- (`self.Health`) Damage)))
  (if (<= _output_get 0)
    (`/Game/Blueprints/ScoreBoard.Add Score` (`self.Score`) (`self.Point Value`))
    (`GameplayStatics.SpawnSoundAtLocation` "/Game/Audio/DeepExplosion_Cue.DeepExplosion_Cue" (`SceneComponent.K2_GetComponentLocation` (`self.Sphere`)) (struct) 1.0 1.0 0.0 null null)
    (`GameplayStatics.SpawnEmitterAtLocation` "/Game/Particles/P_Explosion.P_Explosion" (`SceneComponent.K2_GetComponentLocation` (`self.Sphere`)) (struct) (2.0 2.0 2.0))
    (`self.K2_DestroyActor`)
    (else
      (`GameplayStatics.SpawnSoundAtLocation` "/Game/Audio/Explosion_Cue.Explosion_Cue" (`SceneComponent.K2_GetComponentLocation` (`self.Sphere`)) (struct) 1.0 1.0 0.0 null null))))

(event `self.SkeletalMesh.OnComponentBeginOverlap`
  (params (OverlappedComponent :type "PrimitiveComponent Object Reference") (OtherActor :type "Actor Object Reference") (OtherComp :type "PrimitiveComponent Object Reference") (OtherBodyIndex :type Integer) (bFromSweep :type Boolean) (SweepResult :type "HitResult Structure (by ref)")))

(event `self.Sphere.OnComponentBeginOverlap`
  (params (OverlappedComponent :type "PrimitiveComponent Object Reference") (OtherActor :type "Actor Object Reference") (OtherComp :type "PrimitiveComponent Object Reference") (OtherBodyIndex :type Integer) (bFromSweep :type Boolean) (SweepResult :type "HitResult Structure (by ref)"))
  ;[1 1 1] Rock hits goal post
  (bind _asship_goal_postl (cast `/Game/Blueprints/ShipGoalPostl` OtherActor))
  (if (`ActorComponent.ComponentHasTag` OtherComp "Damagable")
    (`/Game/Blueprints/ShipGoalPostl.Update health` _asship_goal_postl (* (`self.Damage Value`) -1))
    (`self.K2_DestroyActor`)))

(fn `OnRep_Damage Value`)

(fn `UserConstructionScript`
  (`parent.UserConstructionScript`))