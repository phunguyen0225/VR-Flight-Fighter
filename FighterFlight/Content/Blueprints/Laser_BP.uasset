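; Laser beam actor that damages Moving_Asteroid actors tagged Destructible while overlapping them.
; Each Tick, a forward Visibility line trace sets the Niagara beam's end and positions the impact effect, shown only on a hit.
; Distance snaps to the hit point, then regrows very rapidly toward MaxDistance each frame.
; Damage comes from overlap events rather than the trace, repeating through a Delay loop until IsDamaging clears on end overlap.
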(event `self.ReceiveBeginPlay`
  (`FXSystemComponent.SetColorParameter` (`self.NiagaraLaser`) "Color" (struct :`R` 1.0 :`G` 0.189166 :`B` 0.039292 :`A` 1.0))
  (`FXSystemComponent.SetColorParameter` (`self.NiagaraLaserImpact`) "Color" (struct :`R` 1.0 :`G` 0.189166 :`B` 0.039292 :`A` 1.0)))

(event `self.ReceiveActorBeginOverlap`
  (params (OtherActor :type "Actor Object Reference"))
  (if (`self.ActorHasTag` OtherActor "Destructible")
    (bind _asmoving_asteroid (cast `/Game/Blueprints/Moving_Asteroid` OtherActor))
    (set `self.IsDamaging` true)
    (`/Game/Blueprints/Moving_Asteroid.Damage Rock` _asmoving_asteroid (`self.Damage`) :!label _label)
    (`KismetSystemLibrary.Delay` 0.2)
    (if (`self.IsDamaging`)
      (goto _label))))

(event `self.ReceiveActorEndOverlap`
  (params (OtherActor :type "Actor Object Reference"))
  (if (`self.ActorHasTag` OtherActor "Destructible")
    (cast `/Game/Blueprints/Moving_Asteroid` OtherActor)
    (set `self.IsDamaging` false)))

(event `self.ReceiveTick`
  (params (DeltaSeconds :type "Float (single-precision)"))
  (bind _returnvalue (`self.K2_GetActorLocation`))
  (bind _returnvalue_2 (+ _returnvalue (* (`self.GetActorForwardVector`) (`self.Distance`))))
  (`|ExecutionSequence`
    (:`then_0`
      (set `self.TraceEnd` _returnvalue_2)
      (bind _outhit (`KismetSystemLibrary.LineTraceSingle` _returnvalue _returnvalue_2 "TraceTypeQuery1"))
      (bind (_bblockinghit _binitialoverlap _time _distance _location) (`GameplayStatics.BreakHitResult` _outhit))
      (set `self.bHit` _bblockinghit)
      (set `self.HitLocation` _location)
      (`FXSystemComponent.SetVectorParameter` (`self.NiagaraLaser`) "LaserEnd" (select `bool` (`self.bHit`) :`false` (`self.TraceEnd`) :`true` (`self.HitLocation`)))
      (`SceneComponent.SetVisibility` (`self.NiagaraLaserImpact`) (`self.bHit`) false)
      (`SceneComponent.K2_SetWorldLocation` (`self.NiagaraLaserImpact`) (`self.HitLocation`) false false)
      (if (`self.bHit`)
        (set `self.Distance` (`KismetMathLibrary.VSize` (- (`self.HitLocation`) (`self.K2_GetActorLocation`))))))
    (:`then_1`
      (if (< (`self.Distance`) (`self.MaxDistance`))
        (set `self.Distance` (+ (`self.Distance`) (* DeltaSeconds 100000000.0)))))))

(fn `UserConstructionScript`)