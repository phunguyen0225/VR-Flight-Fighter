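; Enemy ship actor for a VR game that flies toward the player Ship and shoots at it.
; On BeginPlay it aims its projectile movement at the Ship with a random speed and turns to face it.
; Tick polls distance through a delay-gated flag; within WaitDistance it stops and spawns EnemyProjectile from GunLocation about once a second.
; Tick also destroys it when VRGameMode reports a loss.
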(event `self.ReceiveBeginPlay`
  (`parent.ReceiveBeginPlay`)
  (`KismetSystemLibrary.Delay` 0.02)
  (set `MovementComponent.Velocity` (* (`KismetMathLibrary.Normal` (- (`self.K2_GetActorLocation` (`self.Ship`)) (`self.K2_GetActorLocation`))) (`KismetMathLibrary.RandomFloatInRange` 90.0 180.0)) (`self.ProjectileMovement`))
  (`self.K2_SetActorRotation` (`KismetMathLibrary.FindLookAtRotation` (`self.K2_GetActorLocation`) (`SceneComponent.K2_GetComponentLocation` (`/Game/Blueprints/ShipGoalPostl.StaticMesh` (`self.Ship`))))))

(event `self.ReceiveTick`
  (params (DeltaSeconds :type "Float (single-precision)"))
  (bind (_returnvalue_x _returnvalue_y _returnvalue_z) (`KismetMathLibrary.BreakVector` (`self.K2_GetActorLocation`)))
  (bind (_returnvalue_x_2 _returnvalue_y_2 _returnvalue_z_2) (`KismetMathLibrary.BreakVector` (`self.K2_GetActorLocation` (`self.Ship`))))
  (`parent.ReceiveTick` DeltaSeconds)
  (`|ExecutionSequence`
    (:`then_0`
      (`KismetSystemLibrary.Delay` 0.2)
      (bind _asvrgame_mode (cast `/Game/VRTemplate/Blueprints/VRGameMode` (`GameplayStatics.GetGameMode`)))
      (if (`/Game/VRTemplate/Blueprints/VRGameMode.IsLose?` _asvrgame_mode)
        (`self.K2_DestroyActor`)))
    (:`then_1`
      (if (`self.Check`)
        (if (> (`KismetMathLibrary.Sqrt` (+ (+ (`KismetMathLibrary.Square` (- _returnvalue_x_2 _returnvalue_x)) (`KismetMathLibrary.Square` (- _returnvalue_y_2 _returnvalue_y))) (`KismetMathLibrary.Square` (- _returnvalue_z_2 _returnvalue_z)))) (`self.WaitDistance`))
          (set `self.Check` false)
          (`KismetSystemLibrary.Delay` 0.2)
          (set `self.Check` true)
          (else
            (`|ExecutionSequence`
              (:`then_0`
                (`/Engine/EditorBlueprintResources/StandardMacros.DoOnce` false
                  (:`Completed`
                    (set `MovementComponent.Velocity` (0.0 0.0 0.0) (`self.ProjectileMovement`))
                    (`KismetSystemLibrary.Delay` 0.1))))
              (:`then_1`
                (`self.Shoot At Ship`)))))))))

(event `Shoot At Ship`
  (set `self.Check` false)
  (`|SpawnActorFromClass` "/Game/Blueprints/EnemyProjectile.EnemyProjectile_C" (`SceneComponent.K2_GetComponentToWorld` (`self.Gun Location`)) "Undefined" "OverrideRootScale" null null)
  (`KismetSystemLibrary.Delay` 1.0)
  (set `self.Check` true))

(fn `UserConstructionScript`
  (`parent.UserConstructionScript`))