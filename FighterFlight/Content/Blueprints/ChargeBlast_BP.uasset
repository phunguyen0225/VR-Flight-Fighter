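; ChargeBlast is a charged projectile that bursts into an Explosion_BP when it overlaps a Destructible-tagged Enemy_Base.
; It passes ChargeScale to the explosion as ChargeFactor, spawning it small below a charge threshold and scaled up with charge otherwise, then destroys itself.
; Other overlaps with physics-simulating components apply a velocity-based impulse and destroy the projectile.
; The timed self-destroy is disconnected and never runs.
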(event `self.SphereCollision.OnComponentBeginOverlap`
  (params (OverlappedComponent :type "PrimitiveComponent Object Reference") (OtherActor :type "Actor Object Reference") (OtherComp :type "PrimitiveComponent Object Reference") (OtherBodyIndex :type Integer) (bFromSweep :type Boolean) (SweepResult :type "HitResult Structure (by ref)"))
  (bind _spherecollision (`self.SphereCollision`))
  (bind _spherecollision_2 (`self.SphereCollision`))
  (if (`self.ActorHasTag` OtherActor "Destructible")
    (cast `/Game/Blueprints/Enemy_Base` OtherActor
      (:`then`
        (if (< (`self.ChargeScale`) 2.0)
          (`|SpawnActorFromClass` "/Game/Blueprints/Explosion_BP.Explosion_BP_C" (`KismetMathLibrary.MakeTransform` (`SceneComponent.K2_GetComponentLocation` _spherecollision) (`SceneComponent.K2_GetComponentRotation` _spherecollision) (0.1 0.1 0.1)) "Undefined" "OverrideRootScale" null (`self.ChargeScale`) null)
          (`KismetSystemLibrary.PrintString` "LESS THAN")
          (else
            (`|SpawnActorFromClass` "/Game/Blueprints/Explosion_BP.Explosion_BP_C" (`KismetMathLibrary.MakeTransform` (`SceneComponent.K2_GetComponentLocation` _spherecollision_2) (`SceneComponent.K2_GetComponentRotation` _spherecollision_2) (* (0.1 0.1 0.1) (* 20 (`self.ChargeScale`)))) "Undefined" "OverrideRootScale" null (`self.ChargeScale`) null)))
        (`self.K2_DestroyActor` :!label _label))
      (:`CastFailed`
        (if (`SceneComponent.IsSimulatingPhysics` OtherComp "None") :!label _label_2
          (`PrimitiveComponent.AddImpulse` OtherComp (* (`MovementComponent.Velocity` (`self.ProjectileMovement`)) 1.0) "None" false)
          (goto _label))))
    (else
      (goto _label_2))))

(event `self.ReceiveBeginPlay`)

(fn `UserConstructionScript`)