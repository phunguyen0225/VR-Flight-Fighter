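; Wave spawner that runs escalating rounds of enemies in a VR game with asteroids and a ship.
; Reset clears spawners, asteroids, score and round board, then starts a delayed Countdown that advances the round and calls BeginWave.
; BeginWave and QuickLoop switch random spawners and raise the capped spawn count, with QuickLoop re-entering Countdown.
; Tick clears the Run flag on game-mode loss; direct-spawning SpawnGroup is deprecated and unused.
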(event `self.ReceiveBeginPlay`)

(event `self.ReceiveTick`
  (params (DeltaSeconds :type "Float (single-precision)"))
  (`KismetSystemLibrary.Delay` 0.2)
  (bind _asvrgame_mode (cast `/Game/VRTemplate/Blueprints/VRGameMode` (`GameplayStatics.GetGameMode`)))
  (if (`/Game/VRTemplate/Blueprints/VRGameMode.IsLose?` _asvrgame_mode)
    (set `self.run` false)))

(event `Reset`
  (`self.Stop Spawning`)
  (set `self.Round` 0)
  (set `self.NumSpawns` 2)
  (set `self.run` true)
  (`/Game/Blueprints/Round_Board.Reset` (`self.Round Board`))
  (`/Game/Blueprints/ScoreBoard.Reset Score` (`self.Score`))
  (for _array_element (`self.Asteroids`)
    (if (`KismetSystemLibrary.IsValid` _array_element)
      (`self.K2_DestroyActor` _array_element)))
  (`self.Countdown`))

(event `Countdown`
  (`KismetSystemLibrary.Delay` 10.0)
  (`/Engine/EditorBlueprintResources/StandardMacros.IncrementInt` (`self.Round`)
    (:`  `
      (if true
        (`/Game/Blueprints/Round_Board.Update Round` (`self.Round Board`) (`self.Round`))
        (`self.Begin Wave`)))))

(event `Begin Wave`
  (bind _numspawns (`self.NumSpawns`))
  (`|ExecutionSequence`
    (:`then_0`
      (`/Engine/EditorBlueprintResources/StandardMacros.IncrementInt` (`self.Counter`) :!label _label
        (:`  `
          (`self.QuickLoop`))))
    (:`then_1`
      (if (`self.run`) :!label _label_2
        (`KismetSystemLibrary.Delay` (`KismetMathLibrary.RandomFloatInRange` 10.0 15.0))
        (goto _label)))
    (:`then_2`
      (goto _label_2))
    (:`then_3`
      (goto _label_2))
    (:`then_4`
      (goto _label_2))
    (:`then_5`
      (goto _label_2))
    (:`then_6`
      (`KismetSystemLibrary.Delay` 10.0)
      (if (<= _numspawns 10)
        (`/Engine/EditorBlueprintResources/StandardMacros.IncrementInt` _numspawns)
        (else
          (while (`KismetArrayLibrary.Array_IsValidIndex` (`self.Asteroids`))
            _)
          (if (`self.run`)
            (`self.End Round`)))))))

(event `Spawn Group`
  (bind _spawners (`self.Spawners`))
  ;[1 1 1] Deprecated
  (for _ (range (+ (`self.NumSpawns`) 1))
    (bind _returnvalue (`|SpawnActorFromClass` "/Game/Blueprints/Enemy_Base.Enemy_Base_C" (`self.GetTransform` (`|GetArrayItem` _spawners (`KismetMathLibrary.RandomIntegerInRange` 0 (`KismetArrayLibrary.Array_LastIndex` _spawners)))) "AdjustIfPossibleButAlwaysSpawn" "OverrideRootScale" null null))
    (set `/Game/Blueprints/Enemy_Base.Ship` (`self.ShipBoard`) _returnvalue)
    (set `/Game/Blueprints/Enemy_Base.Score` (`self.Score`) _returnvalue)
    (`KismetArrayLibrary.Array_Add` (`self.Asteroids`) _returnvalue)))

(event `QuickLoop`
  (bind _spawners (`self.Spawners`))
  (bind _numspawns (`self.NumSpawns`))
  ;[1 1 1] Deprecated
  (for _ (range (+ (`self.NumSpawns`) 1))
    (`/Game/Blueprints/AsteroidSpawner.Switchspawning` (`|GetArrayItem` _spawners (`KismetMathLibrary.RandomIntegerInRange` 0 (`KismetArrayLibrary.Array_LastIndex` _spawners)))))
  (`KismetSystemLibrary.Delay` 1.0)
  (if (<= _numspawns 10)
    (`/Engine/EditorBlueprintResources/StandardMacros.IncrementInt` _numspawns
      (:`  `
        _)))
  (`self.Countdown`))

(event `End Round`
  (if (`self.run`)
    (`self.Countdown`)))

(event `Stop Spawning`
  (for _array_element (`self.Spawners`)
    (`/Game/Blueprints/AsteroidSpawner.Don't SPawn` _array_element)))

(fn `UserConstructionScript`)