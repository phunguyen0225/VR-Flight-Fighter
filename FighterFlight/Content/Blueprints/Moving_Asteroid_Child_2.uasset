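; Moving asteroid child Blueprint for a VR game, launched toward the ship's position with a random tumble.
; After a brief delay on BeginPlay, it sets projectile velocity once toward the ship at random speed and randomizes rotation rate on all three axes.
; Tick, gated by a short Delay, checks the VRGameMode lose flag and destroys the asteroid when the game is lost.
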(event `self.ReceiveBeginPlay`
  (`parent.ReceiveBeginPlay`)
  (`KismetSystemLibrary.Delay` 0.02)
  (set `MovementComponent.Velocity` (* (`KismetMathLibrary.Normal` (- (`self.K2_GetActorLocation` (`self.Ship`)) (`self.K2_GetActorLocation`))) (`KismetMathLibrary.RandomFloatInRange` 90.0 180.0)) (`self.ProjectileMovement`))
  (set `RotatingMovementComponent.RotationRate` (`KismetMathLibrary.MakeRotator` (`KismetMathLibrary.RandomFloatInRange` 10.0 90.0) (`KismetMathLibrary.RandomFloatInRange` 10.0 90.0) (`KismetMathLibrary.RandomFloatInRange` 10.0 90.0)) (`self.RotatingMovement`)))

(event `self.ReceiveTick`
  (params (DeltaSeconds :type "Float (single-precision)"))
  (`parent.ReceiveTick` DeltaSeconds)
  (`KismetSystemLibrary.Delay` 0.2)
  (bind _asvrgame_mode (cast `/Game/VRTemplate/Blueprints/VRGameMode` (`GameplayStatics.GetGameMode`)))
  (if (`/Game/VRTemplate/Blueprints/VRGameMode.IsLose?` _asvrgame_mode)
    (`self.K2_DestroyActor`)))

(fn `UserConstructionScript`
  (`parent.UserConstructionScript`))