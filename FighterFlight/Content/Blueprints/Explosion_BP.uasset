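; Explosion actor that damages Moving_Asteroid actors it overlaps, scaled by a charge factor.
; An overlap with a Destructible-tagged actor casts it to Moving_Asteroid and calls DamageRock with truncated BaseDamage times ChargeFactor.
; After debug prints and a one-second delay it destroys itself, which happens only following such a hit.
; The particle activation is disconnected and never runs.
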(event `self.ReceiveBeginPlay`)

(event `self.ReceiveActorBeginOverlap`
  (params (OtherActor :type "Actor Object Reference"))
  (bind _chargefactor (`self.ChargeFactor`))
  (bind _returnvalue (`KismetStringLibrary.Conv_DoubleToString` _chargefactor))
  (if (`self.ActorHasTag` OtherActor "Destructible")
    (bind _asmoving_asteroid (cast `/Game/Blueprints/Moving_Asteroid` OtherActor))
    (`/Game/Blueprints/Moving_Asteroid.Damage Rock` _asmoving_asteroid (`KismetMathLibrary.FTrunc` (* (`self.BaseDamage`) _chargefactor)))
    (`KismetSystemLibrary.PrintString` "Explosion Scale")
    (`KismetSystemLibrary.PrintString` _returnvalue)
    (`KismetSystemLibrary.Delay` 1.0)
    (`KismetSystemLibrary.PrintString` _returnvalue)
    (`KismetSystemLibrary.PrintString` "Hello")
    (`self.K2_DestroyActor`)))

(fn `UserConstructionScript`)