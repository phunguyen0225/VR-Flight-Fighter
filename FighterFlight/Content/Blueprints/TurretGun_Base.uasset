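; TurretGun_Base is a turret gun actor whose aim follows a separate TurretController.
; CheckRotation and ClientcheckRotation share one path that, while the controller is grabbed, rotates the gun toward its LookAtLocation.
; Otherwise a timeline lerps the gun back to the transform saved at BeginPlay.
; Nothing live here calls either event: Tick is empty and a delayed CheckRotation call is disconnected.
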(event `self.ReceiveBeginPlay`
  (set `self.default position` (`self.GetTransform`)))

(event `self.ReceiveTick`
  (params (DeltaSeconds :type "Float (single-precision)")))

(event `Check Rotation`
  (if (`/Game/Blueprints/Turret_joystick_2.IsGrabbed?` (`self.Turret Controller`)) :!label _label
    (`self.K2_SetActorRotation` (`KismetMathLibrary.FindLookAtRotation` (`self.K2_GetActorLocation`) (`/Game/Blueprints/Turret_joystick_2.Look at Location` (`self.Turret Controller`))))
    (else
      (`Timeline|Timeline_0` :!via `PlayFromStart`
        (:`Update`
          (`self.K2_SetActorTransform` (`KismetMathLibrary.TLerp` (`self.GetTransform`) (`self.default position`))))))))

(event `Client check Rotation`
  (goto _label))

(fn `UserConstructionScript`)