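; Enemy ship Blueprint that sets its own health and flies a randomized, endlessly looping box-shaped patrol.
; BeginPlay calls the parent, then drives ProjectileMovement through local forward, down, backward and up velocities.
; A self-looping Delay chain replaces Tick, re-rolling speed and duration on each leg, with shorter vertical legs, so the path varies and can drift.
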(event `self.ReceiveBeginPlay`
  (`parent.ReceiveBeginPlay`)
  (set `self.Health` 15)
  (`ProjectileMovementComponent.SetVelocityInLocalSpace` (`self.ProjectileMovement`) (* (1.0 0.0 0.0) (`KismetMathLibrary.RandomFloatInRange` 1200.0 2000.0)) :!label _label)
  (`KismetSystemLibrary.Delay` (`KismetMathLibrary.RandomFloatInRange` 1.0 2.0))
  (`ProjectileMovementComponent.SetVelocityInLocalSpace` (`self.ProjectileMovement`) (* (0.0 0.0 -1.0) (`KismetMathLibrary.RandomFloatInRange` 1200.0 2000.0)))
  (`KismetSystemLibrary.Delay` (`KismetMathLibrary.RandomFloatInRange` 0.5 1.0))
  (`ProjectileMovementComponent.SetVelocityInLocalSpace` (`self.ProjectileMovement`) (* (-1.0 0.0 0.0) (`KismetMathLibrary.RandomFloatInRange` 1200.0 2000.0)))
  (`KismetSystemLibrary.Delay` (`KismetMathLibrary.RandomFloatInRange` 1.0 2.0))
  (`ProjectileMovementComponent.SetVelocityInLocalSpace` (`self.ProjectileMovement`) (* (0.0 0.0 1.0) (`KismetMathLibrary.RandomFloatInRange` 1200.0 2000.0)))
  (`KismetSystemLibrary.Delay` (`KismetMathLibrary.RandomFloatInRange` 0.5 1.0))
  (goto _label))

(fn `UserConstructionScript`
  (`parent.UserConstructionScript`))