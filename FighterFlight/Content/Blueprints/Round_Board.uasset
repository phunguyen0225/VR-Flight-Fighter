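; Round_Board is a display actor that shows the current round number through a RoundDisplay user widget held in its Widget component.
; UpdateRound casts the component's widget to RoundDisplay and sets its text to "Round" joined directly to the number, with no space.
; Reset forwards to the widget's own Reset, and the board has no active tick, overlap or construction logic.
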(event `Update Round`
  (params (Round :type Integer))
  (bind _asround_display (cast `/Game/Blueprints/RoundDisplay` (`WidgetComponent.GetUserWidgetObject` (`self.Widget`))))
  (`/Game/Blueprints/RoundDisplay.Set Text` _asround_display (`KismetTextLibrary.Conv_StringToText` (`KismetStringLibrary.Concat_StrStr` "Round " (`KismetStringLibrary.Conv_IntToString` Round)))))

(event `Reset`
  (bind _asround_display (cast `/Game/Blueprints/RoundDisplay` (`WidgetComponent.GetUserWidgetObject` (`self.Widget`))))
  (`/Game/Blueprints/RoundDisplay.Reset` _asround_display))

(fn `UserConstructionScript`)