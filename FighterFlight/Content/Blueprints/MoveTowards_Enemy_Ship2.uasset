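; Enemy ship in a VR game that weaves toward the player's Ship, then stops within WaitDistance to shoot at it.
; A recursive delayed event swings ProjectileMovement velocity between Right and Left component directions on top of a random-speed approach velocity.
; Tick checks distance, ends the weave loop once in range and spawns aimed EnemyProjectiles, throttled by the Check flag.
; It destroys itself when VRGameMode reports a loss; an unconnected box-pattern movement loop remains unused.
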(event `self.ReceiveBeginPlay`
  (bind _returnvalue (* (`KismetMathLibrary.Normal` (- (`self.K2_GetActorLocation` (`self.Ship`)) (`self.K2_GetActorLocation`))) (`KismetMathLibrary.RandomFloatInRange` 90.0 180.0)))
  (`parent.ReceiveBeginPlay`)
  (set `self.Health` 15)
  (`KismetSystemLibrary.Delay` 0.02)
  (set `MovementComponent.Velocity` _returnvalue (`self.ProjectileMovement`))
  (set `self.Velocity Base` _returnvalue)
  (`self.Back And Forth Movement`))

(event `Back And Forth Movement`
  (bind _projectilemovement (`self.ProjectileMovement`))
  (if (`self.Loop`)
    (set `MovementComponent.Velocity` (+ (`self.Velocity Base`) (* (`SceneComponent.GetForwardVector` (`self.Right`)) 1000.0)) _projectilemovement)
    (`KismetSystemLibrary.Delay` 2.0)
    (if true
      (set `MovementComponent.Velocity` (+ (`self.Velocity Base`) (* (`SceneComponent.GetForwardVector` (`self.Left`)) 1000.0)) _projectilemovement)
      (`KismetSystemLibrary.Delay` 2.0)
      (`self.Back And Forth Movement`))))

(event `self.ReceiveTick`
  (params (DeltaSeconds :type "Float (single-precision)"))
  (bind (_returnvalue_x _returnvalue_y _returnvalue_z) (`KismetMathLibrary.BreakVector` (`self.K2_GetActorLocation`)))
  (bind (_returnvalue_x_2 _returnvalue_y_2 _returnvalue_z_2) (`KismetMathLibrary.BreakVector` (`self.K2_GetActorLocation` (`self.Ship`))))
  (`parent.ReceiveTick` DeltaSeconds)
  (`|ExecutionSequence`
    (:`then_0`
      (`KismetSystemLibrary.Delay` 0.2)
      (bind _asvrgame_mode (cast `/Game/VRTemplate/Blueprints/VRGameMode` (`GameplayStatics.GetGameMode`)))
      (if (`/Game/VRTemplate/Blueprints/VRGameMode.IsLose?` _asvrgame_mode)
        (`self.K2_DestroyActor`)))
    (:`then_1`
      (if (`self.Check`)
        (if (> (`KismetMathLibrary.Sqrt` (+ (+ (`KismetMathLibrary.Square` (- _returnvalue_x_2 _returnvalue_x)) (`KismetMathLibrary.Square` (- _returnvalue_y_2 _returnvalue_y))) (`KismetMathLibrary.Square` (- _returnvalue_z_2 _returnvalue_z)))) (`self.Wait Distance`))
          (set `self.Check` false)
          (`KismetSystemLibrary.Delay` 0.2)
          (set `self.Check` true)
          (else
            (`|ExecutionSequence`
              (:`then_0`
                (`/Engine/EditorBlueprintResources/StandardMacros.DoOnce` false
                  (:`Completed`
                    (set `MovementComponent.Velocity` (0.0 0.0 0.0) (`self.ProjectileMovement`))
                    (set `self.Loop` false)
                    (`KismetSystemLibrary.Delay` 0.2))))
              (:`then_1`
                (`self.Shoot At Ship`)))))))))

(event `Shoot At Ship`
  (bind _returnvalue (`SceneComponent.K2_GetComponentLocation` (`self.Muzzle Location`)))
  (set `self.Check` false)
  (`|SpawnActorFromClass` "/Game/Blueprints/EnemyProjectile.EnemyProjectile_C" (`KismetMathLibrary.MakeTransform` _returnvalue (`KismetMathLibrary.FindLookAtRotation` _returnvalue (`self.K2_GetActorLocation` (`self.Ship`)))) "AdjustIfPossibleButAlwaysSpawn" "OverrideRootScale" null null)
  (`KismetSystemLibrary.Delay` 1.0)
  (set `self.Check` true))

(fn `UserConstructionScript`
  (`parent.UserConstructionScript`))