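; Grabbable VR joystick that aims and fires a linked turret gun, with haptics, sounds and weapon-coloured glow.
; While held, a looping controller line trace sets LookAtLocation for the turret's rotation; dropping it stops firing and cycles standard, laser and charge weapons.
; Each weapon has its own graph, spending HUD-displayed ammo, plus a super variant during the timed PowerUp, which refills ammo.
; Most actions branch on authority into server or client-named events.
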(event `self.ReceiveBeginPlay`
  (set `self.default position` (`self.GetTransform`)))

(event `Glow Up`
  ;[1 1 1] Turret Lights On
  (if (> (`self.Ammo`) 0) :!label _label
    (if (`self.Powerup`)
      (`PrimitiveComponent.SetMaterial` (`/Game/Blueprints/TurretGun_Base.Cannon` (`self.Turret_Gun`)) 0 "/Game/Materials/Glow/GlowBox.GlowBox")
      (`PrimitiveComponent.SetMaterial` (`/Game/Blueprints/TurretGun_Base.secondary1` (`self.Turret_Gun`)) 0 "/Game/Materials/Glow/GlowBox.GlowBox")
      (`PrimitiveComponent.SetMaterial` (`/Game/Blueprints/TurretGun_Base.secondary2` (`self.Turret_Gun`)) 0 "/Game/Materials/Glow/GlowBox.GlowBox")
      (`PrimitiveComponent.SetMaterial` (`/Game/Blueprints/TurretGun_Base.base` (`self.Turret_Gun`)) 0 "/Game/Materials/Glow/GlowTurret.GlowTurret")
      (else
        (switch `int` (`self.WeaponType`)
          (:`1`
            (`PrimitiveComponent.SetMaterial` (`/Game/Blueprints/TurretGun_Base.Cannon` (`self.Turret_Gun`)) 0 "/Game/Materials/Glow/GlowBoxYellow.GlowBoxYellow")
            (`PrimitiveComponent.SetMaterial` (`/Game/Blueprints/TurretGun_Base.secondary1` (`self.Turret_Gun`)) 0 "/Game/Materials/Glow/GlowBoxYellow.GlowBoxYellow")
            (`PrimitiveComponent.SetMaterial` (`/Game/Blueprints/TurretGun_Base.secondary2` (`self.Turret_Gun`)) 0 "/Game/Materials/Glow/GlowBoxYellow.GlowBoxYellow")
            (`PrimitiveComponent.SetMaterial` (`/Game/Blueprints/TurretGun_Base.base` (`self.Turret_Gun`)) 0 "/Game/Materials/Glow/GlowTurretYellow.GlowTurretYellow"))
          (:`2`
            (`PrimitiveComponent.SetMaterial` (`/Game/Blueprints/TurretGun_Base.Cannon` (`self.Turret_Gun`)) 0 "/Game/Materials/Glow/GlowBoxRed.GlowBoxRed")
            (`PrimitiveComponent.SetMaterial` (`/Game/Blueprints/TurretGun_Base.secondary1` (`self.Turret_Gun`)) 0 "/Game/Materials/Glow/GlowBoxRed.GlowBoxRed")
            (`PrimitiveComponent.SetMaterial` (`/Game/Blueprints/TurretGun_Base.secondary2` (`self.Turret_Gun`)) 0 "/Game/Materials/Glow/GlowBoxRed.GlowBoxRed")
            (`PrimitiveComponent.SetMaterial` (`/Game/Blueprints/TurretGun_Base.base` (`self.Turret_Gun`)) 0 "/Game/Materials/Glow/GlowTurretRed.GlowTurretRed"))
          (:`3`
            (`PrimitiveComponent.SetMaterial` (`/Game/Blueprints/TurretGun_Base.Cannon` (`self.Turret_Gun`)) 0 "/Game/Materials/Glow/GlowBoxPurple.GlowBoxPurple")
            (`PrimitiveComponent.SetMaterial` (`/Game/Blueprints/TurretGun_Base.secondary1` (`self.Turret_Gun`)) 0 "/Game/Materials/Glow/GlowBoxPurple.GlowBoxPurple")
            (`PrimitiveComponent.SetMaterial` (`/Game/Blueprints/TurretGun_Base.secondary2` (`self.Turret_Gun`)) 0 "/Game/Materials/Glow/GlowBoxPurple.GlowBoxPurple")
            (`PrimitiveComponent.SetMaterial` (`/Game/Blueprints/TurretGun_Base.base` (`self.Turret_Gun`)) 0 "/Game/Materials/Glow/GlowTurretPurple.GlowTurretPurple")))))))

(event `self.GrabComponent.OnGrabbed`
  ;[1 1 1] Grab
  (set `self.IsGrabbed?` true)
  (`/Engine/EditorBlueprintResources/ActorMacros.Switch Has Authority`
    (:`Authority`
      (`self.Find Controller Point Location`))
    (:`Remote`
      (`self.Client Find Controller Point Location`)))
  (`GameplayStatics.PlaySoundAtLocation` "/Game/Audio/lightsaberon_Cue.lightsaberon_Cue" (`SceneComponent.K2_GetComponentLocation` (`self.GrabComponent`)) (struct) 1.0 1.0 0.0 null null null)
  (`/Engine/EditorBlueprintResources/ActorMacros.Switch Has Authority`
    (:`Authority`
      (`self.Glow Up`))
    (:`Remote`
      (`self.Client Glow Up`)))
  (`PlayerController.PlayHapticEffect` (`GameplayStatics.GetPlayerController` 0) null (select `bool` (== (`MotionControllerComponent.MotionSource` (`/Game/VRTemplate/Blueprints/GrabComponent.MotionControllerRef` (`self.GrabComponent`))) "Left") :`false` "Right" :`true` "Left" :!type "EControllerHand Enum") 1.0 false))

(event `Client Glow Up`
  ;[1 1 1] Turret Lights On
  (goto _label))

(event `self.GrabComponent.OnDropped`
  ;[1 1 1] Drop
  (`PrimitiveComponent.SetMaterial` (`/Game/Blueprints/TurretGun_Base.Cannon` (`self.Turret_Gun`)) 0 "/Game/Materials/GlowyBase.GlowyBase")
  (`PrimitiveComponent.SetMaterial` (`/Game/Blueprints/TurretGun_Base.secondary1` (`self.Turret_Gun`)) 0 "/Game/Materials/GlowyBase.GlowyBase")
  (`PrimitiveComponent.SetMaterial` (`/Game/Blueprints/TurretGun_Base.secondary2` (`self.Turret_Gun`)) 0 "/Game/Materials/GlowyBase.GlowyBase")
  (`PrimitiveComponent.SetMaterial` (`/Game/Blueprints/TurretGun_Base.base` (`self.Turret_Gun`)) 0 "/Game/Materials/GlowyBase.GlowyBase")
  (`/Engine/EditorBlueprintResources/ActorMacros.Switch Has Authority`
    (:`Authority`
      (`self.Server Automatic Release`)
      (`self.Switch Type`))
    (:`Remote`
      (`self.Client Trigger Release`)
      (`self.Client Switch Type`)))
  (set `self.IsGrabbed?` false))

(event `Find Controller Point Location`
  (bind _returnvalue (`SceneComponent.K2_GetComponentLocation` (`self.Grabbing Controller`)))
  (bind _returnvalue_2 (+ _returnvalue (* (`SceneComponent.GetForwardVector` (`self.Grabbing Controller`)) 5000)))
  ;[1 1 1] Line Trace
  (`KismetSystemLibrary.Delay` 0.01 :!label _label_2)
  (if (`self.IsGrabbed?`)
    (bind (_outhit _returnvalue_3) (`KismetSystemLibrary.LineTraceSingle` :`Start` _returnvalue :`End` _returnvalue_2 :`TraceChannel` "TraceTypeQuery1" :`DrawDebugType` "ForOneFrame"))
    (if _returnvalue_3
      (set `self.Look at Location` (`.Location` (`GameplayStatics.BreakHitResult` _outhit)))
      (else
        (set `self.Look at Location` _returnvalue_2)))
    (`/Game/Blueprints/TurretGun_Base.Check Rotation` (`self.Turret_Gun`))
    (`KismetSystemLibrary.Delay` 0.016667)
    (`/Engine/EditorBlueprintResources/ActorMacros.Switch Has Authority`
      (:`Authority`
        (`self.Find Controller Point Location`))
      (:`Remote`
        (`self.Client Find Controller Point Location`)))))

(event `Client Find Controller Point Location`
  ;[1 1 1] Line Trace
  (goto _label_2))

(event `self.TriggerPressed`
  ;[1 1 1] Fire Trigger
  (if (`self.Powerup`)
    (switch `int` (`self.WeaponType`)
      (:`1`
        (set `self.IsFiring` true)
        (`/Engine/EditorBlueprintResources/ActorMacros.Switch Has Authority`
          (:`Authority`
            (`self.Fire Standard SUPER`))
          (:`Remote`
            (`self.Client Fire Standard SUPER`))))
      (:`2`
        (set `self.IsFiring` true)
        (`/Engine/EditorBlueprintResources/ActorMacros.Switch Has Authority`
          (:`Authority`
            (`self.Fire Laser SUPER`))
          (:`Remote`
            (`self.Client Fire Laser SUPER`))))
      (:`3`
        (set `self.IsCharging` true)
        (`/Engine/EditorBlueprintResources/ActorMacros.Switch Has Authority`
          (:`Authority`
            (`self.Fire Charge Super`)))))
    (else
      (switch `int` (`self.WeaponType`)
        (:`1`
          (set `self.IsFiring` true)
          (`/Engine/EditorBlueprintResources/ActorMacros.Switch Has Authority`
            (:`Authority`
              (`self.FireStandard`))
            (:`Remote`
              (`self.Client FireStandard`))))
        (:`2`
          (set `self.IsFiring` true)
          (`/Engine/EditorBlueprintResources/ActorMacros.Switch Has Authority`
            (:`Authority`
              (`self.Fire Laser`))
            (:`Remote`
              (`self.Client Fire Laser`))))
        (:`3`
          (set `self.IsCharging` true)
          (`/Engine/EditorBlueprintResources/ActorMacros.Switch Has Authority`
            (:`Authority`
              (`self.Fire Charge`))
            (:`Remote`
              (`self.Client Fire Charge`))))))))

(event `self.TriggerReleased`
  (bind _superlaser (`self.SuperLaser`))
  (bind _laser (`self.Laser`))
  ;[1 1 1] Release Fire Trigger
  (switch `int` (`self.WeaponType`) :!label _label_3
    (:`Default`
      (set `self.IsFiring` false))
    (:`1`
      (set `self.IsFiring` false))
    (:`2`
      (set `self.IsFiring` false)
      (if (`self.Powerup`)
        (if (`KismetSystemLibrary.IsValid` _superlaser)
          (`/Engine/EditorBlueprintResources/ActorMacros.Switch Has Authority`
            (:`Authority`
              (`/Game/Blueprints/Laser_OP_BP.Server End Beam` _superlaser))
            (:`Remote`
              (`/Game/Blueprints/Laser_OP_BP.Client End Beam` _superlaser)))
          (`AudioComponent.Stop` (`self.BeamSound`) :!label _label_4))
        (elif (`KismetSystemLibrary.IsValid` _laser)
          (`/Engine/EditorBlueprintResources/ActorMacros.Switch Has Authority`
            (:`Authority`
              (`/Game/Blueprints/Laser_BP.Server End Beam` _laser)
              (goto _label_4))
            (:`Remote`
              (`/Game/Blueprints/Laser_BP.Client End Beam` _laser)
              (goto _label_4))))))
    (:`3`
      (set `self.IsCharging` false))))

(event `Server Automatic Release`
  ;[1 1 1] Release Fire Trigger
  (goto _label_3))

(event `Client Trigger Release`
  ;[1 1 1] Release Fire Trigger
  (goto _label_3))

(event `Switch Type`
  ;[1 1 1] Switch Weapon Type
  (if (== (`self.WeaponType`) (`self.WeaponTypeMax`)) :!label _label_5
    (set `self.WeaponType` 1)
    (else
      (`/Engine/EditorBlueprintResources/StandardMacros.IncrementInt` (`self.WeaponType`)))))

(event `Client Switch Type`
  ;[1 1 1] Switch Weapon Type
  (goto _label_5))

(event `Update Ammo`
  (params (Subtract :type Integer))
  ;[1 1 1] Ammo Update
  (set `self.Ammo` (- (`self.Ammo`) Subtract))
  (bind _ashud (cast `/Game/ui/HUD` (`WidgetComponent.GetWidget` (`self.AmmoWidget`))))
  (set `/Game/ui/HUD.AmmoPercentageLeft` (/ (`KismetMathLibrary.Conv_IntToDouble` (`self.Ammo`)) (`KismetMathLibrary.Conv_IntToDouble` (`self.MaxAmmo`))) _ashud))

(event `Power Up`
  (`self.TriggerReleased`)
  (if (> (`self.PowerupJuice`) 0)
    (set `self.PowerupJuice` (- (`self.PowerupJuice`) 1))
    (set `self.Ammo` (`self.MaxAmmo`))
    (set `self.Powerup` true)
    (`GameplayStatics.PlaySoundAtLocation` null (`SceneComponent.K2_GetComponentLocation` (`self.StaticMesh`)) (struct) 1.0 1.0 0.0 null null null)
    (`self.Glow Up`)
    (`KismetSystemLibrary.Delay` 12.0)
    (`self.TriggerReleased`)
    (set `self.Powerup` false)
    (`self.Glow Up`)))

(event `FireStandard`
  (bind _muzzlelocation (`/Game/Blueprints/TurretGun_Base.MuzzleLocation` (`self.Turret_Gun`)))
  (bind _returnvalue (`SceneComponent.K2_GetComponentLocation` _muzzlelocation))
  ;[0 0.809 1] Fire Standard Gun
  (if (> (`self.Ammo`) 0) :!label _label
    (`|SpawnActorFromClass` "/Game/Blueprints/OurProjectile.OurProjectile_C" (`KismetMathLibrary.MakeTransform` _returnvalue (`SceneComponent.K2_GetComponentRotation` _muzzlelocation)) "Undefined" "OverrideRootScale" null null)
    (`self.Update Ammo` 4)
    (`PlayerController.PlayHapticEffect` (`GameplayStatics.GetPlayerController` 0) (`self.PistolFireHapticEffect`) (select `bool` (== (`MotionControllerComponent.MotionSource` (`/Game/VRTemplate/Blueprints/GrabComponent.MotionControllerRef` (`self.GrabComponent`))) "Left") :`false` "Right" :`true` "Left" :!type "EControllerHand Enum") 1.0 false)
    (`GameplayStatics.PlaySoundAtLocation` "/Game/Audio/Arwing.Arwing" (`SceneComponent.K2_GetComponentLocation` (`/Game/Blueprints/TurretGun_Base.MuzzleLocation` (`self.Turret_Gun`))) (struct) 1.0 1.0 0.1 null null null)
    (`KismetSystemLibrary.Delay` 0.2)
    (if (`self.IsFiring`)
      (`self.FireStandard`))
    (else
      (`GameplayStatics.PlaySoundAtLocation` null _returnvalue (struct) 1.0 1.0 0.0 null null null)
      (`PrimitiveComponent.SetMaterial` (`/Game/Blueprints/TurretGun_Base.Cannon` (`self.Turret_Gun`)) 0 "/Game/Materials/GlowyBase.GlowyBase")
      (`PrimitiveComponent.SetMaterial` (`/Game/Blueprints/TurretGun_Base.secondary1` (`self.Turret_Gun`)) 0 "/Game/Materials/GlowyBase.GlowyBase")
      (`PrimitiveComponent.SetMaterial` (`/Game/Blueprints/TurretGun_Base.secondary2` (`self.Turret_Gun`)) 0 "/Game/Materials/GlowyBase.GlowyBase")
      (`PrimitiveComponent.SetMaterial` (`/Game/Blueprints/TurretGun_Base.base` (`self.Turret_Gun`)) 0 "/Game/Materials/GlowyBase.GlowyBase"))))

(event `Client FireStandard`
  ;[0 0.809 1] Fire Standard Gun
  (goto _label))

(event `Fire Standard SUPER`
  (bind _muzzlelocation (`/Game/Blueprints/TurretGun_Base.MuzzleLocation` (`self.Turret_Gun`)))
  (`|SpawnActorFromClass` "/Game/Blueprints/OurProjectileSUPER.OurProjectileSUPER_C" (`KismetMathLibrary.MakeTransform` (`SceneComponent.K2_GetComponentLocation` _muzzlelocation) (`SceneComponent.K2_GetComponentRotation` _muzzlelocation)) "Undefined" "OverrideRootScale" null null :!label _label_2)
  (`PlayerController.PlayHapticEffect` (`GameplayStatics.GetPlayerController` 0) (`self.PistolFireHapticEffect`) (select `bool` (== (`MotionControllerComponent.MotionSource` (`/Game/VRTemplate/Blueprints/GrabComponent.MotionControllerRef` (`self.GrabComponent`))) "Left") :`false` "Right" :`true` "Left" :!type "EControllerHand Enum") 1.0 false)
  (`GameplayStatics.PlaySoundAtLocation` "/Game/Audio/Arwing.Arwing" (`SceneComponent.K2_GetComponentLocation` (`/Game/Blueprints/TurretGun_Base.MuzzleLocation` (`self.Turret_Gun`))) (struct) 1.0 1.0 0.1 null null null)
  (`KismetSystemLibrary.Delay` 0.1)
  (if (`self.IsFiring`)
    (`self.FireStandard`)))

(event `Client Fire Standard SUPER`
  (goto _label_2))

(event `Fire Laser`
  (bind _muzzlelocation (`/Game/Blueprints/TurretGun_Base.MuzzleLocation` (`self.Turret_Gun`)))
  (bind _muzzlelocation_2 (`/Game/Blueprints/TurretGun_Base.MuzzleLocation` (`self.Turret_Gun`)))
  (bind _returnvalue (`SceneComponent.K2_GetComponentLocation` _muzzlelocation))
  ;[1 1 1] Fire Laser
  (if (> (`self.Ammo`) 0) :!label _label
    (bind _returnvalue_2 (`|SpawnActorFromClass` "/Game/Blueprints/Laser_BP.Laser_BP_C" (`KismetMathLibrary.MakeTransform` _returnvalue (`SceneComponent.K2_GetComponentRotation` _muzzlelocation)) "Undefined" "OverrideRootScale" null null))
    (bind _output_get (set `self.Laser` _returnvalue_2))
    (`self.K2_AttachToComponent` _output_get _muzzlelocation_2 "None" "SnapToTarget" "SnapToTarget" "KeepRelative" true)
    (bind _returnvalue_3 (`GameplayStatics.SpawnSoundAttached` "/Game/Audio/ContinuousLaserSound_Cue.ContinuousLaserSound_Cue" _muzzlelocation_2 "None" (0.0 0.0 0.0) (struct) "KeepRelativeOffset" false 1.0 1.0 0.0 null null))
    (set `self.BeamSound` _returnvalue_3)
    (if (and (> (`self.Ammo`) 0) (`self.IsFiring`)) :!label _label_2
      (`self.Update Ammo` 2)
      (`KismetSystemLibrary.Delay` 0.2)
      (goto _label_2)
      (elif (not (> (`self.Ammo`) 0))
        (`self.TriggerReleased`)))
    (else
      (`GameplayStatics.PlaySoundAtLocation` null _returnvalue (struct) 1.0 1.0 0.0 null null null)
      (`PrimitiveComponent.SetMaterial` (`/Game/Blueprints/TurretGun_Base.Cannon` (`self.Turret_Gun`)) 0 "/Game/Materials/GlowyBase.GlowyBase")
      (`PrimitiveComponent.SetMaterial` (`/Game/Blueprints/TurretGun_Base.secondary1` (`self.Turret_Gun`)) 0 "/Game/Materials/GlowyBase.GlowyBase")
      (`PrimitiveComponent.SetMaterial` (`/Game/Blueprints/TurretGun_Base.secondary2` (`self.Turret_Gun`)) 0 "/Game/Materials/GlowyBase.GlowyBase")
      (`PrimitiveComponent.SetMaterial` (`/Game/Blueprints/TurretGun_Base.base` (`self.Turret_Gun`)) 0 "/Game/Materials/GlowyBase.GlowyBase"))))

(event `Client Fire Laser`
  ;[1 1 1] Fire Laser
  (goto _label))

(event `Fire Laser SUPER`
  (bind _muzzlelocation (`/Game/Blueprints/TurretGun_Base.MuzzleLocation` (`self.Turret_Gun`)))
  (bind _muzzlelocation_2 (`/Game/Blueprints/TurretGun_Base.MuzzleLocation` (`self.Turret_Gun`)))
  (bind _returnvalue (`|SpawnActorFromClass` "/Game/Blueprints/Laser_OP_BP.Laser_OP_BP_C" (`KismetMathLibrary.MakeTransform` (`SceneComponent.K2_GetComponentLocation` _muzzlelocation) (`SceneComponent.K2_GetComponentRotation` _muzzlelocation)) "Undefined" "OverrideRootScale" null null :!label _label_3))
  (bind _output_get (set `self.SuperLaser` _returnvalue))
  (`self.K2_AttachToComponent` _output_get _muzzlelocation_2 "None" "SnapToTarget" "SnapToTarget" "KeepRelative" true)
  (bind _returnvalue_2 (`GameplayStatics.SpawnSoundAttached` "/Game/Audio/ContinuousLaserSound_Cue.ContinuousLaserSound_Cue" _muzzlelocation_2 "None" (0.0 0.0 0.0) (struct) "KeepRelativeOffset" false 1.0 1.0 0.0 null null))
  (set `self.BeamSound` _returnvalue_2))

(event `Client Fire Laser SUPER`
  (goto _label_3))

(event `Fire Charge`
  (bind _muzzlelocation (`/Game/Blueprints/TurretGun_Base.MuzzleLocation` (`self.Turret_Gun`)))
  (bind _returnvalue (`SceneComponent.K2_GetComponentLocation` _muzzlelocation))
  (bind _returnvalue_2 (`SceneComponent.K2_GetComponentScale` (`/Game/Blueprints/ChargeBlast_BP.StaticMesh` (`self.SpawnedBlast`))))
  ;[1 1 1] Fire Trigger - Charge Energy
  (if (> (`self.Ammo`) 0) :!label _label
    (`self.Update Ammo` 20)
    (bind _returnvalue_3 (`GameplayStatics.SpawnSoundAtLocation` "/Game/Audio/StarshipRailgunCharge_Cue.StarshipRailgunCharge_Cue" _returnvalue (struct) 1.0 1.0 0.0 null null))
    (set `self.ChargeSound` _returnvalue_3)
    (bind _returnvalue_4 (`|SpawnActorFromClass` "/Game/Blueprints/ChargeBlast_BP.ChargeBlast_BP_C" (`KismetMathLibrary.MakeTransform` _returnvalue (`KismetMathLibrary.NegateRotator` (`SceneComponent.K2_GetComponentRotation` _muzzlelocation))) "Undefined" "OverrideRootScale" null null))
    (bind _output_get (set `self.SpawnedBlast` _returnvalue_4))
    (`ProjectileMovementComponent.SetVelocityInLocalSpace` (`/Game/Blueprints/ChargeBlast_BP.ProjectileMovement` _output_get) (0.0 0.0 0.0))
    (`self.K2_AttachToComponent` (`self.SpawnedBlast`) (`/Game/Blueprints/TurretGun_Base.MuzzleLocation` (`self.Turret_Gun`)) "None" "SnapToTarget" "SnapToTarget" "KeepRelative" true)
    (if (`self.IsCharging`) :!label _label_2
      (if (== _returnvalue_2 (`self.MaxSizeScale`) :`ErrorTolerance` 0.01)
        (set `/Game/Blueprints/ChargeBlast_BP.ChargeScale` (`self.ChargeScale`) (`self.SpawnedBlast`))
        (`/Engine/EditorBlueprintResources/ActorMacros.Switch Has Authority`
          (:`Authority`
            (`self.Blast Charge`))
          (:`Remote`
            (`self.Client Blast Charge`)))
        (else
          (`SceneComponent.SetWorldScale3D` (`/Game/Blueprints/ChargeBlast_BP.StaticMesh` (`self.SpawnedBlast`)) (+ _returnvalue_2 0.01))
          (set `self.ChargeScale` (+ (`self.ChargeScale`) 0.03))
          (`KismetSystemLibrary.Delay` 0.01)
          (goto _label_2)))
      (else
        (set `/Game/Blueprints/ChargeBlast_BP.ChargeScale` (`self.ChargeScale`) (`self.SpawnedBlast`))
        (`/Engine/EditorBlueprintResources/ActorMacros.Switch Has Authority`
          (:`Authority`
            (`self.Blast Charge`))
          (:`Remote`
            (`self.Client Blast Charge`)))))
    (else
      (`GameplayStatics.PlaySoundAtLocation` null _returnvalue (struct) 1.0 1.0 0.0 null null null)
      (`PrimitiveComponent.SetMaterial` (`/Game/Blueprints/TurretGun_Base.Cannon` (`self.Turret_Gun`)) 0 "/Game/Materials/GlowyBase.GlowyBase")
      (`PrimitiveComponent.SetMaterial` (`/Game/Blueprints/TurretGun_Base.secondary1` (`self.Turret_Gun`)) 0 "/Game/Materials/GlowyBase.GlowyBase")
      (`PrimitiveComponent.SetMaterial` (`/Game/Blueprints/TurretGun_Base.secondary2` (`self.Turret_Gun`)) 0 "/Game/Materials/GlowyBase.GlowyBase")
      (`PrimitiveComponent.SetMaterial` (`/Game/Blueprints/TurretGun_Base.base` (`self.Turret_Gun`)) 0 "/Game/Materials/GlowyBase.GlowyBase"))))

(event `Client Fire Charge`
  ;[1 1 1] Fire Trigger - Charge Energy
  (goto _label))

(event `Blast Charge`
  (bind _spawnedblast (`self.SpawnedBlast`))
  ;[1 1 1] Release Trigger - Blast Projectile
  (`AudioComponent.Stop` (`self.ChargeSound`) :!label _label_3)
  (bind _returnvalue (`GameplayStatics.SpawnSoundAtLocation` "/Game/Audio/StarshipRailgunFire_Cue.StarshipRailgunFire_Cue" (`SceneComponent.K2_GetComponentLocation` (`/Game/Blueprints/TurretGun_Base.MuzzleLocation` (`self.Turret_Gun`))) (struct) 1.0 1.0 0.0 null null))
  (`AudioComponent.StopDelayed` _returnvalue 2.5)
  (`self.K2_DetachFromActor` (`self.SpawnedBlast`) "KeepWorld" "KeepWorld" "KeepRelative")
  (`ProjectileMovementComponent.SetVelocityInLocalSpace` (`/Game/Blueprints/ChargeBlast_BP.ProjectileMovement` (`self.SpawnedBlast`)) (* (1500.0 0.0 0.0) (`self.ChargeScale`)))
  (set `/Game/Blueprints/ChargeBlast_BP.Damage` (`KismetMathLibrary.FTrunc` (* (`/Game/Blueprints/ChargeBlast_BP.Damage` _spawnedblast) (`self.ChargeScale`))) _spawnedblast)
  (set `self.ChargeScale` 1.0))

(event `Client Blast Charge`
  ;[1 1 1] Release Trigger - Blast Projectile
  (goto _label_3))

(event `Fire Charge Super`
  (bind _muzzlelocation (`/Game/Blueprints/TurretGun_Base.MuzzleLocation` (`self.Turret_Gun`)))
  (`|SpawnActorFromClass` "/Game/Blueprints/ChargeBlastSUPER.ChargeBlastSUPER_C" (`KismetMathLibrary.MakeTransform` (`SceneComponent.K2_GetComponentLocation` _muzzlelocation) (`SceneComponent.K2_GetComponentRotation` _muzzlelocation)) "Undefined" "OverrideRootScale" null null :!label _label_4)
  (`PlayerController.PlayHapticEffect` (`GameplayStatics.GetPlayerController` 0) (`self.PistolFireHapticEffect`) (select `bool` (== (`MotionControllerComponent.MotionSource` (`/Game/VRTemplate/Blueprints/GrabComponent.MotionControllerRef` (`self.GrabComponent`))) "Left") :`false` "Right" :`true` "Left" :!type "EControllerHand Enum") 1.0 false)
  (`GameplayStatics.PlaySoundAtLocation` "/Game/Audio/StarshipRailgunFire_Cue.StarshipRailgunFire_Cue" (`SceneComponent.K2_GetComponentLocation` (`/Game/Blueprints/TurretGun_Base.MuzzleLocation` (`self.Turret_Gun`))) (struct) 1.0 1.0 0.1 null null null))

(event `Client FIre Charge Super`
  (goto _label_4))

(fn `NewFunction_0`)

(fn `OnRep_Look at Location`)

(fn `UserConstructionScript`)